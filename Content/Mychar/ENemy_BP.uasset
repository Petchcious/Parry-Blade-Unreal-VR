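; VR melee enemy Blueprint that duels the VRPawn with random light, heavy and unparryable attacks, each timed by montages, delays and hitbox toggles.
; Overlaps resolve shield blocks and blade parries, with directional reactions and counterattacks after parried heavies.
; Parries build a stack that triggers a stun, enabling four directional hitboxes for damaging swings.
; Tick drives attack selection, stun, health bar and death, gated by state booleans.
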(event `AttackRightHeavy`
  (bind _bladehitbox (`self.BladeHitbox`))
  ;[1 0.7104 0.9629] AttackRightHeavy
  (set `self.IsAttacking` true)
  (set `self.HeavyDown` true)
  (`/Engine/EditorBlueprintResources/StandardMacros.DoOnce` false :!label _label
    (:`Completed`
      (`self.PlayAnimMontage` "/Game/Mychar/UseAnim/Montage/Attack/AttackRightHeavy2_Montage.AttackRightHeavy2_Montage")
      (`self.Play Enemy Attack SFX`)
      (`KismetSystemLibrary.PrintString` "HeavyAttackRight")
      (`KismetSystemLibrary.Delay` 1.0)
      (`PrimitiveComponent.SetCollisionEnabled` _bladehitbox "QueryOnly")
      (`self.DodgeCheck`)
      (`KismetSystemLibrary.Delay` 1.0)
      (set `self.IsAttacking` false)
      (set `self.HeavyDown` false)
      (`PrimitiveComponent.SetCollisionEnabled` _bladehitbox "QueryOnly")
      (`self.StopAnimMontage` "/Game/Mychar/UseAnim/Montage/Attack/AttackRightHeavy2_Montage.AttackRightHeavy2_Montage")
      (`self.Knock`)
      (goto _label :!via `Reset`))))

(event `UnParryMove1`
  (bind _rightleghitbox (`self.RightLegHitbox`))
  ;[1 0.4766 0.848] UnparryMove1
  (set `self.IsAttacking` true)
  (set `self.UnParryable` true)
  (`/Engine/EditorBlueprintResources/StandardMacros.DoOnce` false :!label _label_2
    (:`Completed`
      (`self.PlayAnimMontage` "/Game/Mychar/UseAnim/Montage/UnParryable/UnParry1.UnParry1")
      (`self.Play Enemy Attack SFX`)
      (`KismetSystemLibrary.PrintString` "UnParry1")
      (`KismetSystemLibrary.Delay` 0.7)
      (`PrimitiveComponent.SetCollisionEnabled` _rightleghitbox "QueryOnly")
      (`self.DodgeCheck`)
      (`KismetSystemLibrary.Delay` 1.0)
      (`PrimitiveComponent.SetCollisionEnabled` _rightleghitbox "NoCollision")
      (set `self.IsAttacking` false)
      (set `self.UnParryable` false)
      (`self.StopAnimMontage` "/Game/Mychar/UseAnim/Montage/UnParryable/UnParry1.UnParry1")
      (`self.Knock`)
      (goto _label_2 :!via `Reset`))))

(event `AttackLeftHeavy`
  (bind _bladehitbox (`self.BladeHitbox`))
  ;[0.6384 0.7499 1] AttackLeftHeavy
  (set `self.IsAttacking` true)
  (set `self.HeavyCenter` true)
  (`/Engine/EditorBlueprintResources/StandardMacros.DoOnce` false :!label _label_3
    (:`Completed`
      (`self.PlayAnimMontage` "/Game/Mychar/UseAnim/Montage/Attack/AttackLeftHeavy_Montage.AttackLeftHeavy_Montage")
      (`self.Play Enemy Attack SFX`)
      (`KismetSystemLibrary.PrintString` "AtackLeftHeavy")
      (`KismetSystemLibrary.Delay` 1.0)
      (`PrimitiveComponent.SetCollisionEnabled` _bladehitbox "QueryOnly")
      (`self.DodgeCheck`)
      (`KismetSystemLibrary.Delay` 1.0)
      (set `self.IsAttacking` false)
      (set `self.HeavyCenter` false)
      (`PrimitiveComponent.SetCollisionEnabled` _bladehitbox "QueryOnly")
      (`self.StopAnimMontage` "/Game/Mychar/UseAnim/Montage/Attack/AttackLeftHeavy_Montage.AttackLeftHeavy_Montage")
      (`self.Knock`)
      (goto _label_3 :!via `Reset`))))

(event `UnParryMove2`
  (bind _rightleghitbox (`self.RightLegHitbox`))
  ;[0.1786 1 0.8296] UnparryMove2
  (set `self.IsAttacking` true)
  (set `self.UnParryable` true)
  (`/Engine/EditorBlueprintResources/StandardMacros.DoOnce` false :!label _label_4
    (:`Completed`
      (`self.PlayAnimMontage` "/Game/Mychar/UseAnim/Montage/UnParryable/UnParry4.UnParry4")
      (`self.Play Enemy Attack SFX`)
      (`KismetSystemLibrary.PrintString` "UnParry1")
      (`KismetSystemLibrary.Delay` 1.05)
      (`PrimitiveComponent.SetCollisionEnabled` _rightleghitbox "QueryOnly")
      (`self.DodgeCheck`)
      (`KismetSystemLibrary.Delay` 1.0)
      (`PrimitiveComponent.SetCollisionEnabled` _rightleghitbox "NoCollision")
      (set `self.IsAttacking` false)
      (set `self.UnParryable` false)
      (`self.StopAnimMontage` "/Game/Mychar/UseAnim/Montage/UnParryable/UnParry4.UnParry4")
      (`self.Knock`)
      (goto _label_4 :!via `Reset`))))

(event `AttackLeft`
  (bind _bladehitbox (`self.BladeHitbox`))
  ;[1 0.7009 0.4314] AttackLeft
  (set `self.IsAttacking` true)
  (set `self.Left` true)
  (`/Engine/EditorBlueprintResources/StandardMacros.DoOnce` false :!label _label_5
    (:`Completed`
      (`self.PlayAnimMontage` "/Game/Mychar/UseAnim/Montage/Attack/LeftAttack.LeftAttack")
      (`self.Play Enemy Attack SFX`)
      (`KismetSystemLibrary.PrintString` "AtackLeft")
      (`KismetSystemLibrary.Delay` 1.0)
      (`PrimitiveComponent.SetCollisionEnabled` _bladehitbox "QueryOnly")
      (`self.DodgeCheck`)
      (`KismetSystemLibrary.Delay` 1.0)
      (set `self.IsAttacking` false)
      (set `self.Left` false)
      (`PrimitiveComponent.SetCollisionEnabled` _bladehitbox "QueryOnly")
      (`self.StopAnimMontage` "/Game/Mychar/UseAnim/Montage/Attack/LeftAttack.LeftAttack")
      (`self.Knock`)
      (goto _label_5 :!via `Reset`))))

(event `UnParryMove3`
  (bind _lefthandhitbox (`self.LeftHandHitbox`))
  ;[0.4441 0.2294 1] UnparryMove3
  (set `self.IsAttacking` true)
  (set `self.UnParryable` true)
  (`/Engine/EditorBlueprintResources/StandardMacros.DoOnce` false :!label _label_6
    (:`Completed`
      (`self.PlayAnimMontage` "/Game/Mychar/UseAnim/Montage/UnParryable/UnParry3.UnParry3")
      (`self.Play Enemy Attack SFX`)
      (`KismetSystemLibrary.PrintString` "UnParry1")
      (`KismetSystemLibrary.Delay` 1.1)
      (`PrimitiveComponent.SetCollisionEnabled` _lefthandhitbox "QueryOnly")
      (`self.DodgeCheck`)
      (`KismetSystemLibrary.Delay` 1.0)
      (`PrimitiveComponent.SetCollisionEnabled` _lefthandhitbox "NoCollision")
      (set `self.IsAttacking` false)
      (set `self.UnParryable` false)
      (`self.StopAnimMontage` "/Game/Mychar/UseAnim/Montage/UnParryable/UnParry3.UnParry3")
      (`self.Knock`)
      (goto _label_6 :!via `Reset`))))

(event `AttackRight`
  (bind _bladehitbox (`self.BladeHitbox`))
  ;[0.7032 1 0.5462] AttacRight
  (set `self.IsAttacking` true)
  (set `self.Right` true)
  (`/Engine/EditorBlueprintResources/StandardMacros.DoOnce` false :!label _label_7
    (:`Completed`
      (`self.PlayAnimMontage` "/Game/Mychar/UseAnim/Montage/Attack/AttackRight_Montage.AttackRight_Montage")
      (`self.Play Enemy Attack SFX`)
      (`KismetSystemLibrary.PrintString` "AttackRIght")
      (`KismetSystemLibrary.Delay` 0.7)
      (`PrimitiveComponent.SetCollisionEnabled` _bladehitbox "QueryOnly")
      (`self.DodgeCheck`)
      (`KismetSystemLibrary.Delay` 1.0)
      (set `self.IsAttacking` false)
      (set `self.Right` false)
      (`PrimitiveComponent.SetCollisionEnabled` _bladehitbox "QueryOnly")
      (`self.StopAnimMontage` "/Game/Mychar/UseAnim/Montage/Attack/AttackRight_Montage.AttackRight_Montage")
      (`self.Knock`)
      (goto _label_7 :!via `Reset`))))

(event `DodgeCheck`
  ;[1 1 1] Dodge Check
  (bind _asvrpawn (cast `/Game/VRTemplate/Blueprints/VRPawn` (`GameplayStatics.GetPlayerPawn` 0)))
  (if (`self.IsPlayerParry`)
    _
    (elif (not (`/Game/VRTemplate/Blueprints/VRPawn.IsPlayerBeingHit` _asvrpawn))
      (`KismetSystemLibrary.PrintString` "Dodge"))))

(event `AttackCenter`
  (bind _bladehitbox (`self.BladeHitbox`))
  ;[0.1968 1 0.8701] AttackCenter
  (set `self.IsAttacking` true)
  (set `self.Center` true)
  (`KismetSystemLibrary.PrintString` "AttackCenter")
  (`/Engine/EditorBlueprintResources/StandardMacros.DoOnce` false :!label _label_8
    (:`Completed`
      (`self.PlayAnimMontage` "/Game/Mychar/UseAnim/Montage/Attack/AttackCenter_Montage.AttackCenter_Montage")
      (`self.Play Enemy Attack SFX`)
      (`KismetSystemLibrary.Delay` 1.0)
      (`PrimitiveComponent.SetCollisionEnabled` _bladehitbox "QueryOnly")
      (`self.DodgeCheck`)
      (`KismetSystemLibrary.Delay` 1.0)
      (set `self.IsAttacking` false)
      (set `self.Center` false)
      (`PrimitiveComponent.SetCollisionEnabled` _bladehitbox "QueryOnly")
      (`self.StopAnimMontage` "/Game/Mychar/UseAnim/Montage/Attack/AttackCenter_Montage.AttackCenter_Montage")
      (`self.Knock`)
      (goto _label_8 :!via `Reset`))))

(event `Knock`
  ;[0.3217 0.4631 1] Knock Check And Reset
  (set `self.IsKnock` true)
  (if (`self.IsPlayerParry`)
    (`KismetSystemLibrary.Delay` 4.0)
    (else
      (`KismetSystemLibrary.Delay` 1.86)))
  (set `self.IsKnock` false))

(event `self.ReceiveTick`
  (params (DeltaSeconds :type "Float (single-precision)"))
  ;[1 0.7518 0.2891] Every Tick Sequences
  (if (not (`self.IsStarting`))
    (`|ExecutionSequence`
      (:`then_0`
        ;[1 0.007701 0] Check DIe
        (if (`self.IsDie`)
          ;[1 0 0.1986] Die
          (`/Engine/EditorBlueprintResources/StandardMacros.DoOnce` false
            (:`Completed`
              (set `self.IsStun` true)
              (`KismetSystemLibrary.Delay` 7.0)
              (set `self.IsStun` false)
              (`GameplayStatics.PlaySound2D` "/Game/Sounds/Death/TSP_Death_Long08_1.TSP_Death_Long08_1" 1.0 1.0 0.0 null null)
              (`|SpawnActorFromClass` "/Game/Mychar/Effect/Spawn_DeathEffect.Spawn_DeathEffect_C" (`SceneComponent.K2_GetComponentToWorld` (`self.Mesh`)) "Undefined" "MultiplyWithRoot" null null)
              (`KismetSystemLibrary.Delay` 3.0)
              (`self.K2_DestroyActor`)))
          (else
            ;[1 0.2705 0.2904] Check Condition
            (if (`self.IsKnock`)
              _
              (elif (`self.IsAttacking`)
                _
                (elif (not (`self.IsStun`))
                  ;[1 0.166 0.2959] Random Attack
                  (switch `/Game/Mychar/EnemyAttack` (`KismetArrayLibrary.Array_Random` (`self.CurrentAttack`))
                    (:`NewEnumerator0`
                      (`self.AttackCenter`))
                    (:`NewEnumerator1`
                      (`self.AttackRight`))
                    (:`NewEnumerator2`
                      (`self.AttackLeft`))
                    (:`NewEnumerator3`
                      (`self.AttackRightHeavy`))
                    (:`NewEnumerator4`
                      (`self.AttackLeftHeavy`))
                    (:`NewEnumerator5`
                      (`self.UnParryMove1`))
                    (:`NewEnumerator6`
                      (`self.UnParryMove2`))
                    (:`NewEnumerator7`
                      (`self.UnParryMove3`)))))))))
      (:`then_1`
        ;[1 0.8542 0] Check Stun
        (if (>= (`self.Stack`) 10)
          (set `self.IsStun` true)
          (`KismetSystemLibrary.Delay` 5.0)
          (set `self.IsStun` false)
          (set `self.Stack` 0)))
      (:`then_2`
        ;[0.452 1 0.9201] Set Health Bar
        (bind _asenemy_health_bar (cast `/Game/Widget/EnemyHealthBar` (`WidgetComponent.GetWidget` (`self.HealthBar`))))
        (`ProgressBar.SetPercent` (`/Game/Widget/EnemyHealthBar.ProgressBar_0` _asenemy_health_bar) (/ (`self.Health`) 100.0)))
      (:`then_3`
        ;[0.6812 0.3226 1] HealthCheck
        (if (<= (`self.Health`) 0.0)
          (set `self.IsDie` true)))
      (:`then_4`
        (if (`self.IsStun`)
          ;[0.108 1 0] Enable Collision
          (`PrimitiveComponent.SetCollisionEnabled` (`self.UpHitbox`) "QueryOnly")
          (`PrimitiveComponent.SetCollisionEnabled` (`self.RightHitbox`) "QueryOnly")
          (`PrimitiveComponent.SetCollisionEnabled` (`self.DownHitbox`) "QueryOnly")
          (`PrimitiveComponent.SetCollisionEnabled` (`self.LeftHitbox`) "QueryOnly")
          (else
            ;[1 0.02091 0] Disable Collision
            (`PrimitiveComponent.SetCollisionEnabled` (`self.UpHitbox`) "NoCollision")
            (`PrimitiveComponent.SetCollisionEnabled` (`self.RightHitbox`) "NoCollision")
            (`PrimitiveComponent.SetCollisionEnabled` (`self.DownHitbox`) "NoCollision")
            (`PrimitiveComponent.SetCollisionEnabled` (`self.LeftHitbox`) "NoCollision")))))))

(event `self.ReceiveBeginPlay`
  ;[0.02166 0.6963 1] Start Sequence
  (`self.PlayAnimMontage` "/Game/Mychar/UseAnim/StaringFall.StaringFall")
  (`KismetSystemLibrary.Delay` 0.5)
  (`GameplayStatics.PlaySound2D` "/Game/Sounds/taunt/SwordslashStab_Earth_1.SwordslashStab_Earth_1" 1.0 1.0 0.0 null null)
  (`|SpawnActorFromClass` "/Game/Mychar/Effect/Spawn_Particle2.Spawn_Particle2_C" (`SceneComponent.K2_GetComponentToWorld` (`self.Mesh`)) "Undefined" "MultiplyWithRoot" null null)
  (`KismetSystemLibrary.Delay` 1.0)
  (`GameplayStatics.PlaySound2D` "/Game/Sounds/taunt/Ninja_Taunt02_1.Ninja_Taunt02_1" 1.0 1.0 0.0 null null)
  (`KismetSystemLibrary.Delay` 5.0)
  (`self.StopAnimMontage` "/Game/Mychar/UseAnim/StaringFall.StaringFall")
  (set `self.IsStarting` false)
  ;[1 0.6161 0] Disable Hitbox When Starting
  (`PrimitiveComponent.SetCollisionEnabled` (`self.RightLegHitbox`) "NoCollision")
  (`PrimitiveComponent.SetCollisionEnabled` (`self.LeftHandHitbox`) "NoCollision")
  (`PrimitiveComponent.SetCollisionEnabled` (`self.BladeHitbox`) "NoCollision")
  (`PrimitiveComponent.SetCollisionEnabled` (`self.UpHitbox`) "NoCollision")
  (`PrimitiveComponent.SetCollisionEnabled` (`self.RightHitbox`) "NoCollision")
  (`PrimitiveComponent.SetCollisionEnabled` (`self.DownHitbox`) "NoCollision")
  (`PrimitiveComponent.SetCollisionEnabled` (`self.LeftHitbox`) "NoCollision"))

(event `self.LeftHandHitbox.OnComponentBeginOverlap`
  (params (OverlappedComponent :type "PrimitiveComponent Object Reference") (OtherActor :type "Actor Object Reference") (OtherComp :type "PrimitiveComponent Object Reference") (OtherBodyIndex :type Integer) (bFromSweep :type Boolean) (SweepResult :type "HitResult Structure (by ref)"))
  ;[1 0.6052 0.4846] Block Check
  (cast `/Game/Shield/Shield_BP` OtherActor)
  (bind _asvrpawn (cast `/Game/VRTemplate/Blueprints/VRPawn` (`GameplayStatics.GetPlayerPawn` 0) :!label _label_9))
  ;[1 0.9658 0.04048] Block
  (if (`/Game/VRTemplate/Blueprints/VRPawn.IsBlocking` _asvrpawn)
    (`/Engine/EditorBlueprintResources/StandardMacros.DoOnce` false :!label _label_10
      (:`Completed`
        (`self.PlayAnimMontage` "/Game/Mychar/UseAnim/Montage/GetParried/GetPariiedRight_Montage.GetPariiedRight_Montage")
        (`|ExecutionSequence`
          (:`then_0`
            (`PrimitiveComponent.SetCollisionEnabled` (`self.LeftHandHitbox`) "NoCollision")
            (`PrimitiveComponent.SetCollisionEnabled` (`self.RightLegHitbox`) "NoCollision"))
          (:`then_1`
            (`GameplayStatics.PlaySound2D` "/Game/Sounds/Shield/Sword_Shield08_1.Sword_Shield08_1" 1.0 1.0 0.0 null null)
            (`PlayerController.PlayHapticEffect` (`GameplayStatics.GetPlayerController` 0) "/Game/VRTemplate/Haptics/PistolFireHapticEffect.PistolFireHapticEffect" "Left" 5.0 false)
            (`KismetSystemLibrary.Delay` 1.0)
            (set `self.IsKnock` true)
            (`KismetSystemLibrary.Delay` 2.0)
            (set `self.IsKnock` false)
            (`self.StopAnimMontage` "/Game/Mychar/UseAnim/Montage/GetParried/GetPariiedRight_Montage.GetPariiedRight_Montage")
            (goto _label_10 :!via `Reset`)))))))

(event `self.RightLegHitbox.OnComponentBeginOverlap`
  (params (OverlappedComponent :type "PrimitiveComponent Object Reference") (OtherActor :type "Actor Object Reference") (OtherComp :type "PrimitiveComponent Object Reference") (OtherBodyIndex :type Integer) (bFromSweep :type Boolean) (SweepResult :type "HitResult Structure (by ref)"))
  ;[1 0.6052 0.4846] Block Check
  (cast `/Game/Shield/Shield_BP` OtherActor)
  (goto _label_9))

(event `self.BladeHitbox.OnComponentBeginOverlap`
  (params (OverlappedComponent :type "PrimitiveComponent Object Reference") (OtherActor :type "Actor Object Reference") (OtherComp :type "PrimitiveComponent Object Reference") (OtherBodyIndex :type Integer) (bFromSweep :type Boolean) (SweepResult :type "HitResult Structure (by ref)"))
  ;[1 0.6052 0.4846] Block Check
  (`|ExecutionSequence`
    (:`then_0`
      (cast `/Game/Shield/Shield_BP` OtherActor)
      (goto _label_9))
    (:`then_1`
      (cast `/Game/blade/MyBlade_BP` OtherActor)
      (bind _asvrpawn (cast `/Game/VRTemplate/Blueprints/VRPawn` (`GameplayStatics.GetPlayerPawn` 0)))
      ;[1 0.2956 0.7464] Check Condition
      (if (`self.IsStun`)
        _
        (elif (`/Game/VRTemplate/Blueprints/VRPawn.IsSwinging` _asvrpawn)
          (if (not (`self.UnParryable`))
            (set `self.IsPlayerParry` true)
            ;[1 0.5108 0.2984] Add Stack
            (set `self.Stack` (+ (`self.Stack`) 1))
            ;[1 0.865 0.6291] GetParry
            ;;[1 0.1235 0.1732] Center
            (if (`self.Center`)
              (`/Engine/EditorBlueprintResources/StandardMacros.DoOnce` false :!label _label_11
                (:`Completed`
                  (`self.PlayAnimMontage` "/Game/Mychar/UseAnim/Montage/GetParried/GetParried_Montage.GetParried_Montage")
                  (`self.SpawnSoundAndEffect`)
                  (set `self.IsKnock` true)
                  (`KismetSystemLibrary.Delay` 1.0)
                  (`self.StopAnimMontage` "/Game/Mychar/UseAnim/Montage/GetParried/GetParried_Montage.GetParried_Montage")
                  (`KismetSystemLibrary.Delay` 2.0)
                  (set `self.IsPlayerParry` false)
                  (set `self.IsKnock` false)
                  (goto _label_11 :!via `Reset`)))
              (else
                ;;[0.2611 1 0.3895] Right
                (if (`self.Right`)
                  (`/Engine/EditorBlueprintResources/StandardMacros.DoOnce` false :!label _label_12
                    (:`Completed`
                      (`self.PlayAnimMontage` "/Game/Mychar/UseAnim/Montage/GetParried/GetPariiedRight_Montage.GetPariiedRight_Montage")
                      (`self.SpawnSoundAndEffect`)
                      (set `self.IsKnock` true)
                      (`KismetSystemLibrary.Delay` 1.0)
                      (`self.StopAnimMontage` "/Game/Mychar/UseAnim/Montage/GetParried/GetPariiedRight_Montage.GetPariiedRight_Montage")
                      (`KismetSystemLibrary.Delay` 2.0)
                      (set `self.IsPlayerParry` false)
                      (set `self.IsKnock` false)
                      (goto _label_12 :!via `Reset`)))
                  (else
                    ;;[1 0.8528 0.04501] Heavy Center
                    (if (`self.HeavyCenter`)
                      (`/Engine/EditorBlueprintResources/StandardMacros.DoOnce` false :!label _label_13
                        (:`Completed`
                          (`self.PlayAnimMontage` "/Game/Mychar/UseAnim/Montage/GetParried/CounterAttackCenter.CounterAttackCenter")
                          (`self.SpawnSoundAndEffect`)
                          (`KismetSystemLibrary.Delay` 0.3)
                          (set `self.IsPlayerParry` false)
                          (set `self.Center` true)
                          (`KismetSystemLibrary.Delay` 3.0)
                          (set `self.IsAttacking` false)
                          (set `self.Center` false)
                          (`self.StopAnimMontage` "/Game/Mychar/UseAnim/Montage/GetParried/CounterAttackCenter.CounterAttackCenter")
                          (goto _label_13 :!via `Reset`)))
                      (else
                        ;;[0.8632 0.7305 0.04374] HeavyDown
                        (if (`self.HeavyDown`)
                          (`/Engine/EditorBlueprintResources/StandardMacros.DoOnce` false :!label _label_14
                            (:`Completed`
                              (`self.PlayAnimMontage` "/Game/Mychar/UseAnim/Montage/GetParried/GetParryied_HeavyCounter.GetParryied_HeavyCounter")
                              (`self.SpawnSoundAndEffect`)
                              (`KismetSystemLibrary.Delay` 0.3)
                              (set `self.IsPlayerParry` false)
                              (set `self.Right` true)
                              (`KismetSystemLibrary.Delay` 3.0)
                              (set `self.IsAttacking` false)
                              (set `self.Right` false)
                              (`self.StopAnimMontage` "/Game/Mychar/UseAnim/Montage/GetParried/GetParryied_HeavyCounter.GetParryied_HeavyCounter")
                              (goto _label_14 :!via `Reset`)))
                          (else
                            ;;[0.333 1 0.4293] Left
                            (if (`self.Left`)
                              (`/Engine/EditorBlueprintResources/StandardMacros.DoOnce` false :!label _label_15
                                (:`Completed`
                                  (`self.PlayAnimMontage` "/Game/Mychar/UseAnim/Montage/GetParried/GetParryiedLeft_Montage.GetParryiedLeft_Montage")
                                  (`self.SpawnSoundAndEffect`)
                                  (set `self.IsKnock` true)
                                  (`KismetSystemLibrary.Delay` 1.0)
                                  (`self.StopAnimMontage` "/Game/Mychar/UseAnim/Montage/GetParried/GetParryiedLeft_Montage.GetParryiedLeft_Montage")
                                  (`KismetSystemLibrary.Delay` 3.0)
                                  (set `self.IsPlayerParry` false)
                                  (set `self.IsKnock` false)
                                  (goto _label_15 :!via `Reset`))))))))))))))))))

(event `SpawnVisualEffect`
  ;[0 0.6928 1] Set Spawn Visual Effect
  (`|SpawnActorFromClass` "/Game/Mychar/Effect/Spawn_Particle1.Spawn_Particle1_C" (`KismetMathLibrary.Conv_VectorToTransform` (`SceneComponent.K2_GetComponentLocation` (stale `self.BladeHitbox.OnComponentBeginOverlap` OverlappedComponent))) "Undefined" "MultiplyWithRoot" null null))

(event `PlayParrySoundEffects`
  ;[1 0.546 0.2172] SoundEffect
  (switch `/Game/Sounds/ParrySounds` (`KismetArrayLibrary.Array_Random` (`self.SoundEFX`))
    (:`NewEnumerator0`
      (bind _returnvalue (`SceneComponent.K2_GetComponentLocation` (stale `self.BladeHitbox.OnComponentBeginOverlap` OverlappedComponent)))
      (`GameplayStatics.SpawnSoundAtLocation` "/Game/Sounds/SOundAttenua/Parry_High01.Parry_High01" _returnvalue (struct) 1.0 1.0 0.0 null null))
    (:`NewEnumerator1`
      (`GameplayStatics.SpawnSoundAtLocation` "/Game/Sounds/SOundAttenua/Parry_High02.Parry_High02" _returnvalue (struct) 1.0 1.0 0.0 null null))
    (:`NewEnumerator2`
      (`GameplayStatics.SpawnSoundAtLocation` "/Game/Sounds/SOundAttenua/Parry_High03.Parry_High03" _returnvalue (struct) 1.0 1.0 0.0 null null))
    (:`NewEnumerator3`
      (`GameplayStatics.SpawnSoundAtLocation` "/Game/Sounds/SOundAttenua/Parry_High04.Parry_High04" _returnvalue (struct) 1.0 1.0 0.0 null null))
    (:`NewEnumerator5`
      (`GameplayStatics.SpawnSoundAtLocation` "/Game/Sounds/SOundAttenua/Parry_Mid01.Parry_Mid01" _returnvalue (struct) 1.0 1.0 0.0 null null))
    (:`NewEnumerator6`
      (`GameplayStatics.SpawnSoundAtLocation` "/Game/Sounds/SOundAttenua/Parry_Mid03.Parry_Mid03" _returnvalue (struct) 1.0 1.0 0.0 null null))
    (:`NewEnumerator7`
      (`GameplayStatics.SpawnSoundAtLocation` "/Game/Sounds/SOundAttenua/Parry_Mid04.Parry_Mid04" _returnvalue (struct) 1.0 1.0 0.0 null null))
    (:`NewEnumerator8`
      (`GameplayStatics.SpawnSoundAtLocation` "/Game/Sounds/SOundAttenua/Parry_Mid05.Parry_Mid05" _returnvalue (struct) 1.0 1.0 0.0 null null))))

(event `self.RightHitbox.OnComponentBeginOverlap`
  (params (OverlappedComponent :type "PrimitiveComponent Object Reference") (OtherActor :type "Actor Object Reference") (OtherComp :type "PrimitiveComponent Object Reference") (OtherBodyIndex :type Integer) (bFromSweep :type Boolean) (SweepResult :type "HitResult Structure (by ref)"))
  ;[0.5743 0.2682 1] While Stuning Animation
  ;;[1 0 0.03743] Right Hit Box
  (cast `/Game/blade/MyBlade_BP` OtherActor)
  (`self.Check Stun And Set Health Play Sound`)
  (`self.PlayAnimMontage` "/Game/Mychar/UseAnim/Montage/React/ReactLeft.ReactLeft")
  (`self.SpawnVisualEffectStunRight`)
  (`KismetSystemLibrary.Delay` 0.4)
  (set `self.IsBeingHitWhileStun` false))

(event `PlayPainSound`
  ;[0 0.6899 1] PainSound
  (switch `/Game/Sounds/Pain/PainSound` (`KismetArrayLibrary.Array_Random` (`self.PainSound`))
    (:`NewEnumerator0`
      (`GameplayStatics.PlaySound2D` "/Game/Sounds/Pain/TSP_Pain_Large07_1.TSP_Pain_Large07_1" 1.0 1.0 0.0 null null))
    (:`NewEnumerator1`
      (`GameplayStatics.PlaySound2D` "/Game/Sounds/Pain/TSP_Pain_Large08_1.TSP_Pain_Large08_1" 1.0 1.0 0.0 null null))
    (:`NewEnumerator2`
      (`GameplayStatics.PlaySound2D` "/Game/Sounds/Pain/TSP_Pain_Large09_1.TSP_Pain_Large09_1" 1.0 1.0 0.0 null null))
    (:`NewEnumerator3`
      (`GameplayStatics.PlaySound2D` "/Game/Sounds/Pain/TSP_Pain_Small12_1.TSP_Pain_Small12_1" 1.0 1.0 0.0 null null))))

(event `SpawnVisualEffectStunRight`
  ;[0.5743 0.2682 1] While Stuning Animation
  ;;[1 0 0.03743] Right Hit Box
  (`|SpawnActorFromClass` "/Game/Mychar/Effect/Spawn_Particle1.Spawn_Particle1_C" (`KismetMathLibrary.Conv_VectorToTransform` (`SceneComponent.K2_GetComponentLocation` (stale `self.RightHitbox.OnComponentBeginOverlap` OverlappedComponent))) "Undefined" "MultiplyWithRoot" null null))

(event `SpawnSoundAndEffect`
  ;[1 0.2436 0.1739] Spawn Sound And Effect And Haptic
  (`PlayerController.PlayHapticEffect` (`GameplayStatics.GetPlayerController` 0) "/Game/VRTemplate/Haptics/PistolFireHapticEffect.PistolFireHapticEffect" "Right" 5.0 false)
  (`self.Play ParryPain Sound`)
  (`self.PlayParrySoundEffects`)
  (`self.SpawnVisualEffect`))

(event `self.LeftHitbox.OnComponentBeginOverlap`
  (params (OverlappedComponent :type "PrimitiveComponent Object Reference") (OtherActor :type "Actor Object Reference") (OtherComp :type "PrimitiveComponent Object Reference") (OtherBodyIndex :type Integer) (bFromSweep :type Boolean) (SweepResult :type "HitResult Structure (by ref)"))
  ;[0.5743 0.2682 1] While Stuning Animation
  ;;[0 1 1] Left Hit Box
  (cast `/Game/blade/MyBlade_BP` OtherActor)
  (`self.Check Stun And Set Health Play Sound`)
  (`self.PlayAnimMontage` "/Game/Mychar/UseAnim/Montage/React/ReactRight.ReactRight")
  (`self.LeftEffect`)
  (`KismetSystemLibrary.Delay` 0.4)
  (set `self.IsBeingHitWhileStun` false))

(event `Play ParryPain Sound`
  ;[0 0.6899 1] ParryPain
  (switch `/Game/Sounds/ParryPain/ParryPain` (`KismetArrayLibrary.Array_Random` (`self.ParryPainSound`))
    (:`NewEnumerator0`
      (`GameplayStatics.PlaySound2D` "/Game/Sounds/ParryPain/TSP_Parry13_1.TSP_Parry13_1" 1.0 1.0 0.0 null null))
    (:`NewEnumerator1`
      (`GameplayStatics.PlaySound2D` "/Game/Sounds/ParryPain/TSP_Parry16_1.TSP_Parry16_1" 1.0 1.0 0.0 null null))
    (:`NewEnumerator2`
      (`GameplayStatics.PlaySound2D` "/Game/Sounds/ParryPain/TSP_Parry17_1.TSP_Parry17_1" 1.0 1.0 0.0 null null))))

(event `LeftEffect`
  ;[0.5743 0.2682 1] While Stuning Animation
  ;;[0 1 1] Left Hit Box
  (`|SpawnActorFromClass` "/Game/Mychar/Effect/Spawn_Particle1.Spawn_Particle1_C" (`KismetMathLibrary.Conv_VectorToTransform` (`SceneComponent.K2_GetComponentLocation` (stale `self.LeftHitbox.OnComponentBeginOverlap` OverlappedComponent))) "Undefined" "MultiplyWithRoot" null null))

(event `self.UpHitbox.OnComponentBeginOverlap`
  (params (OverlappedComponent :type "PrimitiveComponent Object Reference") (OtherActor :type "Actor Object Reference") (OtherComp :type "PrimitiveComponent Object Reference") (OtherBodyIndex :type Integer) (bFromSweep :type Boolean) (SweepResult :type "HitResult Structure (by ref)"))
  ;[0.5743 0.2682 1] While Stuning Animation
  ;;[0.5165 0 1] Up Hit Box
  (cast `/Game/blade/MyBlade_BP` OtherActor)
  (`self.Check Stun And Set Health Play Sound`)
  (`self.PlayAnimMontage` "/Game/Mychar/UseAnim/Montage/React/ReactDown.ReactDown")
  (`self.UpEffect`)
  (`KismetSystemLibrary.Delay` 0.4)
  (set `self.IsBeingHitWhileStun` false))

(event `Play Enemy Attack SFX`
  (bind _returnvalue (`SceneComponent.K2_GetComponentLocation` (`self.Mesh`)))
  ;[0 0.6899 1] Enemy Attack SFX
  (switch `/Game/Sounds/EnemyAttackSound/EnemyAttackSFX` (`KismetArrayLibrary.Array_Random` (`self.EnemyAttackSFX`))
    (:`NewEnumerator0`
      (`GameplayStatics.SpawnSoundAtLocation` "/Game/Sounds/EnemyAttackSound/EnemyAttackSFX1_Cue.EnemyAttackSFX1_Cue" _returnvalue (struct) 1.0 1.0 0.0 null null))
    (:`NewEnumerator1`
      (`GameplayStatics.SpawnSoundAtLocation` "/Game/Sounds/EnemyAttackSound/EnemyAttackSFX2_Cue.EnemyAttackSFX2_Cue" _returnvalue (struct) 1.0 1.0 0.0 null null))
    (:`NewEnumerator2`
      (`GameplayStatics.SpawnSoundAtLocation` "/Game/Sounds/EnemyAttackSound/EnemyAttackSFX3_Cue.EnemyAttackSFX3_Cue" _returnvalue (struct) 1.0 1.0 0.0 null null))
    (:`NewEnumerator3`
      (`GameplayStatics.SpawnSoundAtLocation` "/Game/Sounds/EnemyAttackSound/EnemyAttackSFX4_Cue.EnemyAttackSFX4_Cue" _returnvalue (struct) 1.0 1.0 0.0 null null))))

(event `UpEffect`
  ;[0.5743 0.2682 1] While Stuning Animation
  ;;[0.5165 0 1] Up Hit Box
  (`|SpawnActorFromClass` "/Game/Mychar/Effect/Spawn_Particle1.Spawn_Particle1_C" (`KismetMathLibrary.Conv_VectorToTransform` (`SceneComponent.K2_GetComponentLocation` (stale `self.UpHitbox.OnComponentBeginOverlap` OverlappedComponent))) "Undefined" "MultiplyWithRoot" null null))

(event `self.DownHitbox.OnComponentBeginOverlap`
  (params (OverlappedComponent :type "PrimitiveComponent Object Reference") (OtherActor :type "Actor Object Reference") (OtherComp :type "PrimitiveComponent Object Reference") (OtherBodyIndex :type Integer) (bFromSweep :type Boolean) (SweepResult :type "HitResult Structure (by ref)"))
  ;[0.5743 0.2682 1] While Stuning Animation
  ;;[0.4904 1 0] Down Hit Box
  (cast `/Game/blade/MyBlade_BP` OtherActor)
  (`self.Check Stun And Set Health Play Sound`)
  (`self.PlayAnimMontage` "/Game/Mychar/UseAnim/Montage/React/ReactUp.ReactUp")
  (`self.DownEffect`)
  (`KismetSystemLibrary.Delay` 0.4)
  (set `self.IsBeingHitWhileStun` false))

(event `DownEffect`
  ;[0.5743 0.2682 1] While Stuning Animation
  ;;[0.4904 1 0] Down Hit Box
  (`|SpawnActorFromClass` "/Game/Mychar/Effect/Spawn_Particle1.Spawn_Particle1_C" (`KismetMathLibrary.Conv_VectorToTransform` (`SceneComponent.K2_GetComponentLocation` (stale `self.DownHitbox.OnComponentBeginOverlap` OverlappedComponent))) "Undefined" "MultiplyWithRoot" null null))

(event `Check Stun And Set Health Play Sound`
  ;[1 0.1329 0.8749] Check Stun Condition Set Health And Play Pain Sound
  (if (`self.IsStun`)
    (if (not (`self.IsBeingHitWhileStun`))
      (bind _asvrpawn (cast `/Game/VRTemplate/Blueprints/VRPawn` (`GameplayStatics.GetPlayerPawn` 0)))
      (if (`/Game/VRTemplate/Blueprints/VRPawn.IsSwinging` _asvrpawn)
        (set `self.IsBeingHitWhileStun` true)
        (set `self.Health` (- (`self.Health`) 5.0))
        (`self.PlayPainSound`)))))

(fn `UserConstructionScript`)