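; VR sword-fighting enemy (Godking montages) that plays an intro, then duels the player with random montage attacks, barks and sounds.
; Tick drives TryAttack, health bar, death and stun, gated by state booleans and Delay cooldowns.
; Blade overlaps resolve shield blocks, player damage and direction-specific parries or counters, with haptics on blocks and parries.
; Stacked parries trigger a stun that opens four directional hitboxes, where swung-blade hits reduce Health.
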(event `Play Dialouge`
  (params (SpeakerName :type String) (CompleteText :type String))
  (bind _aswbp_speech_bubble (cast `/Game/Widgets/WBP_SpeechBubble` (`WidgetComponent.GetWidget` (`self.Dialouge`))))
  (`/Game/Widgets/WBP_SpeechBubble.ShowDialogue` _aswbp_speech_bubble SpeakerName CompleteText)
  (`KismetSystemLibrary.Delay` 3.0)
  (`/Game/Widgets/WBP_SpeechBubble.HideDialogue` _aswbp_speech_bubble))

(event `FinishAttack`
  (set `self.IsAttacking` false)
  (set `self.IsKnock` true))

(event `AttackRightHeavy`
  ;[1 1 1] AttackRightHeavy
  (set `self.IsAttacking` true)
  (set `self.HeavyDown` true)
  (`|PlayMontage` (`self.Mesh`) "/Game/Mychar/GodKingUseAnim/attack/godkingheavyattackdown.godkingheavyattackdown"
    (:`then`
      (`self.Play Enemy Attack SFX`)
      (`self.Play Dialouge` "" "Eat This!!!!")
      (`self.DodgeCheck`))
    (:`OnCompleted`
      (`self.FinishAttack`)
      (set `self.HeavyDown` false))))

(event `AttackLeftHeavy`
  ;[1 1 1] AttackLeftHeavy
  (set `self.IsAttacking` true)
  (set `self.HeavyCenter` true)
  (`|PlayMontage` (`self.Mesh`) "/Game/Mychar/GodKingUseAnim/attack/godkingheavyattackleft.godkingheavyattackleft"
    (:`then`
      (`self.Play Enemy Attack SFX`)
      (`self.Play Dialouge` "" "You Can't dodge this!!!!")
      (`self.DodgeCheck`))
    (:`OnCompleted`
      (`self.FinishAttack`)
      (set `self.HeavyCenter` false))))

(event `AttackLeft`
  ;[1 1 1] AttackLeft
  (set `self.IsAttacking` true)
  (set `self.Left` true)
  (`|PlayMontage` (`self.Mesh`) "/Game/Mychar/GodKingUseAnim/attack/godkingattackleft.godkingattackleft"
    (:`then`
      (`self.Play Enemy Attack SFX`)
      (`self.Play Dialouge` "" "Screww you!!")
      (`self.DodgeCheck`))
    (:`OnCompleted`
      (`self.FinishAttack`)
      (set `self.Left` false))))

(event `UnParryMove1`
  ;[1 1 1] UnparryMove1
  (set `self.IsAttacking` true)
  (set `self.Center` true)
  (`|PlayMontage` (`self.Mesh`) "/Game/Mychar/GodKingUseAnim/moreattack/moreattackcenter.moreattackcenter"
    (:`then`
      (`self.Play Enemy Attack SFX`)
      (`self.Play Dialouge` "" "Too slow!")
      (`self.DodgeCheck`))
    (:`OnCompleted`
      (`self.FinishAttack`)
      (set `self.Center` false))))

(event `AttackRight`
  ;[1 1 1] AttacRight
  (set `self.IsAttacking` true)
  (set `self.Right` true)
  (`|PlayMontage` (`self.Mesh`) "/Game/Mychar/GodKingUseAnim/attack/godking_Right.godking_Right"
    (:`then`
      (`self.Play Enemy Attack SFX`)
      (`self.Play Dialouge` "" "Let's see you handle this")
      (`self.DodgeCheck`))
    (:`OnCompleted`
      (`self.FinishAttack`)
      (set `self.Right` false))))

(event `UnParryMove2`
  ;[1 1 1] UnparryMove2
  (set `self.IsAttacking` true)
  (set `self.Center` true)
  (`|PlayMontage` (`self.Mesh`) "/Game/Mychar/GodKingUseAnim/moreattack/moreattackcenter2.moreattackcenter2"
    (:`then`
      (`self.Play Enemy Attack SFX`)
      (`self.Play Dialouge` "" "Nowhere to run!")
      (`self.DodgeCheck`))
    (:`OnCompleted`
      (`self.FinishAttack`)
      (set `self.Center` false))))

(event `AttackCenter`
  ;[1 1 1] AttackCenter
  (set `self.IsAttacking` true)
  (set `self.Center` true)
  (`|PlayMontage` (`self.Mesh`) "/Game/Mychar/GodKingUseAnim/attack/godkingattackcenter.godkingattackcenter"
    (:`then`
      (`self.Play Enemy Attack SFX`)
      (`self.Play Dialouge` "" "You can't run away from me!!!")
      (`self.DodgeCheck`))
    (:`OnCompleted`
      (`self.FinishAttack`)
      (set `self.Center` false))))

(event `UnParryMove3`
  ;[1 1 1] UnparryMove3
  (set `self.IsAttacking` true)
  (set `self.Center` true)
  (`|PlayMontage` (`self.Mesh`) "/Game/Mychar/GodKingUseAnim/moreattack/moreattackleft.moreattackleft"
    (:`then`
      (`self.Play Enemy Attack SFX`)
      (`self.Play Dialouge` "" "This is the end of the line for you")
      (`self.DodgeCheck`))
    (:`OnCompleted`
      (`self.FinishAttack`)
      (set `self.Center` false))))

(event `self.ReceiveTick`
  (params (DeltaSeconds :type "Float (single-precision)"))
  (if (not (`self.IsStarting`))
    (`|ExecutionSequence`
      (:`then_0`
        (if (`self.IsDie`)
          (`/Engine/EditorBlueprintResources/StandardMacros.DoOnce` false
            (:`Completed`
              (set `self.IsStun` true)
              (`KismetSystemLibrary.Delay` 7.0)
              (set `self.IsStun` false)
              (`GameplayStatics.PlaySound2D` "/Game/EditSounds/DeathSFX_Cue.DeathSFX_Cue" 1.0 1.0 0.0 null null)
              (`|SpawnActorFromClass` "/Game/Mychar/Effect/Spawn_DeathEffect.Spawn_DeathEffect_C" (`SceneComponent.K2_GetComponentToWorld` (`self.Mesh`)) "Undefined" "MultiplyWithRoot" null null)
              (`KismetSystemLibrary.Delay` 3.0)
              (`self.K2_DestroyActor`)))
          (else
            (`self.TryAttack`))))
      (:`then_1`
        (if (>= (`self.Stack`) 4)
          (set `self.IsStun` true)
          (`KismetSystemLibrary.Delay` 5.0)
          (set `self.IsStun` false)
          (set `self.Stack` 0)
          (set `self.IsAttacking` false)
          (set `self.IsKnock` true)))
      (:`then_2`
        (bind _asenemy_health_bar (cast `/Game/Widget/EnemyHealthBar` (`WidgetComponent.GetWidget` (`self.HealthBar`))))
        (`ProgressBar.SetPercent` (`/Game/Widget/EnemyHealthBar.ProgressBar_0` _asenemy_health_bar) (/ (`self.Health`) 100.0)))
      (:`then_3`
        ;[1 1 1] HealthCheck
        (if (<= (`self.Health`) 0.0)
          (set `self.IsDie` true)))
      (:`then_4`
        (if (`self.IsStun`)
          (`PrimitiveComponent.SetCollisionEnabled` (`self.UpHitbox`) "QueryOnly")
          (`PrimitiveComponent.SetCollisionEnabled` (`self.RightHitbox`) "QueryOnly")
          (`PrimitiveComponent.SetCollisionEnabled` (`self.DownHitbox`) "QueryOnly")
          (`PrimitiveComponent.SetCollisionEnabled` (`self.LeftHitbox`) "QueryOnly")
          (else
            (`PrimitiveComponent.SetCollisionEnabled` (`self.UpHitbox`) "NoCollision")
            (`PrimitiveComponent.SetCollisionEnabled` (`self.RightHitbox`) "NoCollision")
            (`PrimitiveComponent.SetCollisionEnabled` (`self.DownHitbox`) "NoCollision")
            (`PrimitiveComponent.SetCollisionEnabled` (`self.LeftHitbox`) "NoCollision"))))
      (:`then_5`
        (if (`self.IsKnock`)
          (`KismetSystemLibrary.Delay` 2.0)
          (set `self.IsKnock` false))))))

(event `self.ReceiveBeginPlay`
  (bind _returnvalue (`GameplayStatics.GetActorOfClass` "/Game/VRTemplate/Blueprints/VRPawn.VRPawn_C"))
  (set `self.VrRef` _returnvalue)
  (`|PlayMontage` (`self.Mesh`) "/Game/Mychar/GodKingUseAnim/opening/godkingopening.godkingopening"
    (:`then`
      (`KismetSystemLibrary.Delay` 0.5)
      (`GameplayStatics.PlaySound2D` "/Game/EditSounds/FirstExplosion.FirstExplosion" 1.0 1.0 0.0 null null)
      (`|SpawnActorFromClass` "/Game/Mychar/Effect/Spawn_Particle2.Spawn_Particle2_C" (`SceneComponent.K2_GetComponentToWorld` (`self.Mesh`)) "Undefined" "MultiplyWithRoot" null null)
      (`KismetSystemLibrary.Delay` 1.0)
      (`GameplayStatics.PlaySound2D` "/Game/EditSounds/FirstLaugh.FirstLaugh" 1.0 1.0 0.0 null null))
    (:`OnCompleted`
      (`self.K2_SetActorLocation` (-576.066441 244.634937 192.564154))
      (`|PlayMontage` (`self.Mesh`) "/Game/Mychar/GodKingUseAnim/GodKing_Walk.GodKing_Walk"
        (:`OnCompleted`
          (set `self.IsStarting` false)
          (`PrimitiveComponent.SetCollisionEnabled` (`self.BladeHitbox`) "NoCollision")
          (`PrimitiveComponent.SetCollisionEnabled` (`self.UpHitbox`) "NoCollision")
          (`PrimitiveComponent.SetCollisionEnabled` (`self.RightHitbox`) "NoCollision")
          (`PrimitiveComponent.SetCollisionEnabled` (`self.DownHitbox`) "NoCollision")
          (`PrimitiveComponent.SetCollisionEnabled` (`self.LeftHitbox`) "NoCollision"))))))

(event `Parry Effects`
  (`self.Play ParryPain Sound`)
  (`self.PlayParrySoundEffects`)
  (`self.SpawnVisualEffect`)
  (`PlayerController.PlayHapticEffect` (`GameplayStatics.GetPlayerController` 0) "/Game/VRTemplate/Haptics/PistolFireHapticEffect.PistolFireHapticEffect" "Right" 5.0 false))

(event `DodgeCheck`
  (bind _asvrpawn (cast `/Game/VRTemplate/Blueprints/VRPawn` (`GameplayStatics.GetPlayerPawn` 0)))
  (if (`self.IsPlayerParry`)
    _
    (elif (not (`/Game/VRTemplate/Blueprints/VRPawn.IsPlayerBeingHit` _asvrpawn))
      (`KismetSystemLibrary.PrintString` "Dodge"))))

(event `self.BladeHitbox.OnComponentBeginOverlap`
  (params (OverlappedComponent :type "PrimitiveComponent Object Reference") (OtherActor :type "Actor Object Reference") (OtherComp :type "PrimitiveComponent Object Reference") (OtherBodyIndex :type Integer) (bFromSweep :type Boolean) (SweepResult :type "HitResult Structure (by ref)"))
  (`|ExecutionSequence`
    (:`then_0`
      (cast `/Game/Shield/Shield_BP` OtherActor)
      (if (`/Game/VRTemplate/Blueprints/VRPawn.IsBlocking` (`self.VrRef`))
        (`|PlayMontage` (`self.Mesh`) "/Game/Mychar/GodKingUseAnim/parry/godkingparrycenter.godkingparrycenter"
          (:`then`
            (`GameplayStatics.PlaySound2D` "/Game/Sounds/Shield/Sword_Shield08_1.Sword_Shield08_1" 1.0 1.0 0.0 null null)
            (`PlayerController.PlayHapticEffect` (`GameplayStatics.GetPlayerController` 0) "/Game/VRTemplate/Haptics/PistolFireHapticEffect.PistolFireHapticEffect" "Left" 5.0 false))
          (:`OnCompleted`
            (set `self.IsKnock` true)
            (set `self.IsAttacking` false)))))
    (:`then_1`
      (bind _asmy_blade_bp (cast `/Game/blade/MyBlade_BP` OtherActor))
      (if (== OtherComp (`/Game/blade/MyBlade_BP.BladeHitBox` _asmy_blade_bp))
        (if (`self.IsStun`)
          _
          (elif (`/Game/VRTemplate/Blueprints/VRPawn.IsSwinging` (`self.VrRef`))
            (if (not (`self.UnParryable`))
              (set `self.IsPlayerParry` true)
              (set `self.Stack` (+ (`self.Stack`) 1))
              ;[1 1 1] GetParry
              (if (`self.Center`)
                (`|PlayMontage` (`self.Mesh`) "/Game/Mychar/GodKingUseAnim/parry/godkingparrycenter.godkingparrycenter"
                  (:`then`
                    (`self.Parry Effects`))
                  (:`OnCompleted`
                    (set `self.IsPlayerParry` false)
                    (set `self.IsKnock` false)
                    (set `self.Center` false)
                    (set `self.IsAttacking` false)))
                (elif (`self.Right`)
                  (`|PlayMontage` (`self.Mesh`) "/Game/Mychar/GodKingUseAnim/parry/godkingparryright.godkingparryright"
                    (:`then`
                      (`self.Parry Effects`))
                    (:`OnCompleted`
                      (set `self.IsPlayerParry` false)
                      (set `self.IsKnock` true)
                      (set `self.Right` false)
                      (set `self.IsAttacking` false)))
                  (elif (`self.Left`)
                    (`|PlayMontage` (`self.Mesh`) "/Game/Mychar/GodKingUseAnim/parry/godkingparryleft.godkingparryleft"
                      (:`then`
                        (`self.Parry Effects`))
                      (:`OnCompleted`
                        (set `self.IsPlayerParry` false)
                        (set `self.IsKnock` true)
                        (set `self.Left` false)
                        (set `self.IsAttacking` false)))
                    (elif (`self.HeavyCenter`)
                      (`|PlayMontage` (`self.Mesh`) "/Game/Mychar/GodKingUseAnim/parry/godkingcountercenter.godkingcountercenter"
                        (:`then`
                          (`self.Parry Effects`)
                          (`KismetSystemLibrary.Delay` 0.1)
                          (set `self.IsPlayerParry` false)
                          (set `self.Center` true))
                        (:`OnCompleted`
                          (set `self.IsAttacking` false)
                          (set `self.Center` true)
                          (set `self.IsKnock` true)))
                      (elif (`self.HeavyDown`)
                        (`|PlayMontage` (`self.Mesh`) "/Game/Mychar/GodKingUseAnim/parry/godkingcounterleft.godkingcounterleft"
                          (:`then`
                            (`self.Parry Effects`)
                            (`KismetSystemLibrary.Delay` 0.1)
                            (set `self.IsPlayerParry` false)
                            (set `self.IsAttacking` true)
                            (set `self.Left` true))
                          (:`OnCompleted`
                            (set `self.IsAttacking` false)
                            (set `self.Left` false)
                            (set `self.IsKnock` true)))))))))))))
    (:`then_2`
      (if (not (`self.IsPlayerParry`))
        (bind _asvrpawn (cast `/Game/VRTemplate/Blueprints/VRPawn` (`GameplayStatics.GetPlayerPawn` 0)))
        (if (== OtherComp (`/Game/VRTemplate/Blueprints/VRPawn.HitboxDetection` _asvrpawn))
          (if (not (`/Game/VRTemplate/Blueprints/VRPawn.IsBlocking` _asvrpawn))
            (`GameplayStatics.ApplyDamage` (`GameplayStatics.GetPlayerPawn` 0) 10.0)))))
    (:`then_3`
      (set `self.SwordLocation` (`SceneComponent.K2_GetComponentLocation` OverlappedComponent)))))

(event `SpawnVisualEffect`
  (`|SpawnActorFromClass` "/Game/Mychar/Effect/Spawn_Particle1.Spawn_Particle1_C" (`KismetMathLibrary.Conv_VectorToTransform` (`SceneComponent.K2_GetComponentLocation` (stale `self.BladeHitbox.OnComponentBeginOverlap` OverlappedComponent))) "Undefined" "MultiplyWithRoot" null null))

(event `PlayPainSound`
  ;[1 1 1] PainSound
  (`GameplayStatics.PlaySound2D` "/Game/EditSounds/PainSFX_Cue.PainSFX_Cue" 1.0 1.0 0.0 null null))

(event `PlayParrySoundEffects`
  ;[1 1 1] SoundEffect
  (`GameplayStatics.SpawnSoundAtLocation` "/Game/EditSounds/Parry_Cue.Parry_Cue" (`self.SwordLocation`) (struct) 1.0 1.0 0.0 null null))

(event `Play ParryPain Sound`
  ;[1 1 1] ParryPain
  (`GameplayStatics.PlaySound2D` "/Game/EditSounds/ParryPainSFX_Cue.ParryPainSFX_Cue" 1.0 1.0 0.0 null null))

(event `SpawnVisualEffectStunRight`
  ;[1 1 1] React Check
  (`|SpawnActorFromClass` "/Game/Mychar/Effect/Spawn_Particle1.Spawn_Particle1_C" (`KismetMathLibrary.Conv_VectorToTransform` (`SceneComponent.K2_GetComponentLocation` (stale `self.RightHitbox.OnComponentBeginOverlap` OverlappedComponent))) "Undefined" "MultiplyWithRoot" null null))

(event `self.RightHitbox.OnComponentBeginOverlap`
  (params (OverlappedComponent :type "PrimitiveComponent Object Reference") (OtherActor :type "Actor Object Reference") (OtherComp :type "PrimitiveComponent Object Reference") (OtherBodyIndex :type Integer) (bFromSweep :type Boolean) (SweepResult :type "HitResult Structure (by ref)"))
  ;[1 1 1] React Check
  (if (`self.IsStun`)
    (if (not (`self.IsBeingHitWhileStun`))
      (cast `/Game/blade/MyBlade_BP` OtherActor)
      (bind _asvrpawn (cast `/Game/VRTemplate/Blueprints/VRPawn` (`GameplayStatics.GetPlayerPawn` 0)))
      (if (`/Game/VRTemplate/Blueprints/VRPawn.IsSwinging` _asvrpawn)
        (set `self.IsBeingHitWhileStun` true)
        (set `self.Health` (- (`self.Health`) 5.0))
        (`self.PlayPainSound`)
        (`self.PlayAnimMontage` "/Game/Mychar/GodKingUseAnim/react/godkingreactleft.godkingreactleft")
        (`self.SpawnVisualEffectStunRight`)
        (`|ExecutionSequence`
          (:`then_0`
            (`KismetSystemLibrary.Delay` 0.4)
            (set `self.IsBeingHitWhileStun` false)))))))

(event `self.LeftHitbox.OnComponentBeginOverlap`
  (params (OverlappedComponent :type "PrimitiveComponent Object Reference") (OtherActor :type "Actor Object Reference") (OtherComp :type "PrimitiveComponent Object Reference") (OtherBodyIndex :type Integer) (bFromSweep :type Boolean) (SweepResult :type "HitResult Structure (by ref)"))
  ;[1 1 1] React Check
  (if (`self.IsStun`)
    (if (not (`self.IsBeingHitWhileStun`))
      (cast `/Game/blade/MyBlade_BP` OtherActor)
      (bind _asvrpawn (cast `/Game/VRTemplate/Blueprints/VRPawn` (`GameplayStatics.GetPlayerPawn` 0)))
      (if (`/Game/VRTemplate/Blueprints/VRPawn.IsSwinging` _asvrpawn)
        (set `self.IsBeingHitWhileStun` true)
        (set `self.Health` (- (`self.Health`) 5.0))
        (`self.PlayPainSound`)
        (`self.PlayAnimMontage` "/Game/Mychar/GodKingUseAnim/react/godkingreactright.godkingreactright")
        (`self.LeftEffect`)
        (`|ExecutionSequence`
          (:`then_0`
            (`KismetSystemLibrary.Delay` 0.4)
            (set `self.IsBeingHitWhileStun` false)))))))

(event `LeftEffect`
  ;[1 1 1] React Check
  (`|SpawnActorFromClass` "/Game/Mychar/Effect/Spawn_Particle1.Spawn_Particle1_C" (`KismetMathLibrary.Conv_VectorToTransform` (`SceneComponent.K2_GetComponentLocation` (stale `self.LeftHitbox.OnComponentBeginOverlap` OverlappedComponent))) "Undefined" "MultiplyWithRoot" null null))

(event `self.UpHitbox.OnComponentBeginOverlap`
  (params (OverlappedComponent :type "PrimitiveComponent Object Reference") (OtherActor :type "Actor Object Reference") (OtherComp :type "PrimitiveComponent Object Reference") (OtherBodyIndex :type Integer) (bFromSweep :type Boolean) (SweepResult :type "HitResult Structure (by ref)"))
  ;[1 1 1] React Check
  (if (`self.IsStun`)
    (if (not (`self.IsBeingHitWhileStun`))
      (cast `/Game/blade/MyBlade_BP` OtherActor)
      (bind _asvrpawn (cast `/Game/VRTemplate/Blueprints/VRPawn` (`GameplayStatics.GetPlayerPawn` 0)))
      (if (`/Game/VRTemplate/Blueprints/VRPawn.IsSwinging` _asvrpawn)
        (set `self.IsBeingHitWhileStun` true)
        (set `self.Health` (- (`self.Health`) 5.0))
        (`self.PlayPainSound`)
        (`self.PlayAnimMontage` "/Game/Mychar/GodKingUseAnim/react/godkingreactdown.godkingreactdown")
        (`self.UpEffect`)
        (`|ExecutionSequence`
          (:`then_0`
            (`KismetSystemLibrary.Delay` 0.4)
            (set `self.IsBeingHitWhileStun` false)))))))

(event `UpEffect`
  ;[1 1 1] React Check
  (`|SpawnActorFromClass` "/Game/Mychar/Effect/Spawn_Particle1.Spawn_Particle1_C" (`KismetMathLibrary.Conv_VectorToTransform` (`SceneComponent.K2_GetComponentLocation` (stale `self.UpHitbox.OnComponentBeginOverlap` OverlappedComponent))) "Undefined" "MultiplyWithRoot" null null))

(event `self.DownHitbox.OnComponentBeginOverlap`
  (params (OverlappedComponent :type "PrimitiveComponent Object Reference") (OtherActor :type "Actor Object Reference") (OtherComp :type "PrimitiveComponent Object Reference") (OtherBodyIndex :type Integer) (bFromSweep :type Boolean) (SweepResult :type "HitResult Structure (by ref)"))
  ;[1 1 1] React Check
  (if (`self.IsStun`)
    (if (not (`self.IsBeingHitWhileStun`))
      (cast `/Game/blade/MyBlade_BP` OtherActor)
      (bind _asvrpawn (cast `/Game/VRTemplate/Blueprints/VRPawn` (`GameplayStatics.GetPlayerPawn` 0)))
      (if (`/Game/VRTemplate/Blueprints/VRPawn.IsSwinging` _asvrpawn)
        (set `self.IsBeingHitWhileStun` true)
        (set `self.Health` (- (`self.Health`) 5.0))
        (`self.PlayPainSound`)
        (`self.PlayAnimMontage` "/Game/Mychar/GodKingUseAnim/react/godkingreactup.godkingreactup")
        (`self.DownEffect`)
        (`|ExecutionSequence`
          (:`then_0`
            (`KismetSystemLibrary.Delay` 0.4)
            (set `self.IsBeingHitWhileStun` false)))))))

(event `DownEffect`
  ;[1 1 1] React Check
  (`|SpawnActorFromClass` "/Game/Mychar/Effect/Spawn_Particle1.Spawn_Particle1_C" (`KismetMathLibrary.Conv_VectorToTransform` (`SceneComponent.K2_GetComponentLocation` (stale `self.DownHitbox.OnComponentBeginOverlap` OverlappedComponent))) "Undefined" "MultiplyWithRoot" null null))

(event `Play Enemy Attack SFX`
  ;[1 1 1] Attack SFX
  (`GameplayStatics.SpawnSoundAtLocation` "/Game/EditSounds/EnemyAttackSFX_Cue.EnemyAttackSFX_Cue" (`SceneComponent.K2_GetComponentLocation` (`self.Mesh`)) (struct) 1.0 1.0 0.0 null null)
  (`self.PlayDialougeSound`))

(event `PlayDialougeSound`
  ;[1 1 1] Dialouge Sound
  (`GameplayStatics.PlaySound2D` "/Game/EditSounds/DialougeSFX_Cue.DialougeSFX_Cue" 1.0 1.0 0.0 null null))

(fn `ParrySound(Old)`
  (switch `/Game/Sounds/ParrySounds` (`KismetArrayLibrary.Array_Random` (`self.SoundEFX`))
    (:`NewEnumerator0`
      (`GameplayStatics.SpawnSoundAtLocation` "/Game/Sounds/SOundAttenua/Parry_High01.Parry_High01" (0.0 0.0 0.0) (struct) 1.0 1.0 0.0 null null))
    (:`NewEnumerator1`
      (`GameplayStatics.SpawnSoundAtLocation` "/Game/Sounds/SOundAttenua/Parry_High02.Parry_High02" (0.0 0.0 0.0) (struct) 1.0 1.0 0.0 null null))
    (:`NewEnumerator2`
      (`GameplayStatics.SpawnSoundAtLocation` "/Game/Sounds/SOundAttenua/Parry_High03.Parry_High03" (0.0 0.0 0.0) (struct) 1.0 1.0 0.0 null null))
    (:`NewEnumerator3`
      (`GameplayStatics.SpawnSoundAtLocation` "/Game/Sounds/SOundAttenua/Parry_High04.Parry_High04" (0.0 0.0 0.0) (struct) 1.0 1.0 0.0 null null))
    (:`NewEnumerator5`
      (`GameplayStatics.SpawnSoundAtLocation` "/Game/Sounds/SOundAttenua/Parry_Mid01.Parry_Mid01" (0.0 0.0 0.0) (struct) 1.0 1.0 0.0 null null))
    (:`NewEnumerator6`
      (`GameplayStatics.SpawnSoundAtLocation` "/Game/Sounds/SOundAttenua/Parry_Mid03.Parry_Mid03" (0.0 0.0 0.0) (struct) 1.0 1.0 0.0 null null))
    (:`NewEnumerator7`
      (`GameplayStatics.SpawnSoundAtLocation` "/Game/Sounds/SOundAttenua/Parry_Mid04.Parry_Mid04" (0.0 0.0 0.0) (struct) 1.0 1.0 0.0 null null))
    (:`NewEnumerator8`
      (`GameplayStatics.SpawnSoundAtLocation` "/Game/Sounds/SOundAttenua/Parry_Mid05.Parry_Mid05" (0.0 0.0 0.0) (struct) 1.0 1.0 0.0 null null))))

(fn `TryAttack`
  (if (`self.IsKnock`)
    _
    (elif (`self.IsAttacking`)
      _
      (elif (not (`self.IsStun`))
        (switch `/Game/Mychar/EnemyAttack` (`KismetArrayLibrary.Array_Random` (`self.CurrentAttack`))
          (:`NewEnumerator0`
            (`self.AttackCenter`))
          (:`NewEnumerator1`
            (`self.AttackRight`))
          (:`NewEnumerator2`
            (`self.AttackLeft`))
          (:`NewEnumerator3`
            (`self.AttackRightHeavy`))
          (:`NewEnumerator4`
            (`self.AttackLeftHeavy`))
          (:`NewEnumerator5`
            (`self.UnParryMove1`))
          (:`NewEnumerator6`
            (`self.UnParryMove2`))
          (:`NewEnumerator7`
            (`self.UnParryMove3`)))))))

(fn `UserConstructionScript`)