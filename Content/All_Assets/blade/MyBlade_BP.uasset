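; MyBlade_BP is a grabbable VR blade that rings and glows.
; From BeginPlay, a delayed loop off the glow timeline's update replays the ring sound and GlowIntensity pulse until the first grab.
; Afterwards, any hit box overlap while the VR pawn is swinging triggers the same sound and a second glow timeline, without checking whether the blade is held.
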(event `self.ReceiveBeginPlay`
  (if (not (`self.FirstGrab`)) :!label _label
    (`self.Play InfBladeSwingRing`)
    (bind (_direction _glowintensity) (`Timeline|Timeline` :!via `PlayFromStart`)
      (:`Update`
        (`MeshComponent.SetScalarParameterValueOnMaterials` (`self.Blade`) "GlowIntensity" _glowintensity)
        (`KismetSystemLibrary.Delay` 2.0)
        (goto _label)))))

(event `self.GrabComponent.OnGrabbed`
  (set `self.FirstGrab` true)
  (set `self.OnGrab` true))

(event `self.GrabComponent.OnDropped`
  (set `self.OnGrab` false))

(event `self.BladeHitBox.OnComponentBeginOverlap`
  (params (OverlappedComponent :type "PrimitiveComponent Object Reference") (OtherActor :type "Actor Object Reference") (OtherComp :type "PrimitiveComponent Object Reference") (OtherBodyIndex :type Integer) (bFromSweep :type Boolean) (SweepResult :type "HitResult Structure (by ref)"))
  (bind _asvrpawn (cast `/Game/VRTemplate/Blueprints/VRPawn` (`GameplayStatics.GetPlayerPawn` 0)))
  (if (`/Game/VRTemplate/Blueprints/VRPawn.IsSwinging` _asvrpawn)
    (`self.Play InfBladeSwingRing`)
    (bind (_direction _glowintensity) (`Timeline|GlowTimeline` :!via `PlayFromStart`)
      (:`Update`
        (`MeshComponent.SetScalarParameterValueOnMaterials` (`self.Blade`) "GlowIntensity" _glowintensity)))))

(event `Play InfBladeSwingRing`
  (`GameplayStatics.SpawnSoundAtLocation` "/Game/EditSounds/INFBladeSwingRing_Cues.INFBladeSwingRing_Cues" (`SceneComponent.K2_GetComponentLocation` (`self.Blade`)) (struct) 1.0 1.0 0.0 null null))

(fn `UserConstructionScript`)